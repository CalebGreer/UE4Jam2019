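; BP_Pawn is a player-controlled pawn that aims and fires charged shots from a barrel.
; On BeginPlay it initializes the BAAiming component with the BAArcDrawer component and its StaticMesh as the barrel.
; The AimAzimuth axis drives Rotate, while pressing Fire starts charging through BAAiming and releasing it fires.
; The Blueprint only wires setup and input, leaving shot logic to BAAiming.
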(event EventBeginPlay
  (Class|BAAimingComponent|Initialize (Variables|Default|GetBAAiming) (Variables|Default|GetBA_ArcDrawer) (Variables|Default|GetStaticMesh)))

(event Collision|EventActorBeginOverlap
  (params (OtherActor :type Actor%20Object%20Reference)))

(event EventTick
  (params (DeltaSeconds :type Float%20%28single-precision%29)))

(event Input|ActionEvents|InputActionFire
  (params (Key :type Key%20Structure))
  (:Pressed
    (Class|BAAimingComponent|ActivateChargingShot (Variables|Default|GetBAAiming)))
  (:Released
    (Class|BAAimingComponent|Fire (Variables|Default|GetBAAiming))))

(event Input|AxisEvents|InputAxisAimAzimuth
  (params (AxisValue :type Float%20%28single-precision%29))
  (Class|BAPawn|Rotate AxisValue))

(fn ConstructionScript)