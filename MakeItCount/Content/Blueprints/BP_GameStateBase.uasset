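; Game state Blueprint that handles level completion by comparing black hole kills with the artifacts in the level.
; Every Tick, while the game mode's NextLevel flag is unset, it finds all BP_BlackHole and BP_Artifact actors.
; When the current artifact count is at most the first black hole's Kills, it opens the hardcoded Level7 and sets NextLevel.
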(event EventTick
  (params (DeltaSeconds :type Float%20%28single-precision%29))
  (bind _asbp_game_mode (Utilities|Casting|CastToBP_GameMode (Game|GetGameMode)))
  (bind _output_get (Variables|Default|SetGameMOde _asbp_game_mode))
  (if (not (Variables|/Game/Blueprints/BP_GameMode.BP_GameMode_C|GetNextLevel _output_get))
    (bind _outactors (Actor|GetAllActorsOfClass "/Game/Blueprints/BP_BlackHole.BP_BlackHole_C"))
    (bind _outactors_2 (Actor|GetAllActorsOfClass "/Game/Blueprints/BP_Artifact.BP_Artifact_C"))
    (bind _output_get_2 (Variables|Default|Settargets (Utilities|Array|Length _outactors_2)))
    (Math|Integer|CompareInt _output_get_2 (Variables|/Script/MakeItCount.BABlackHoleActor|GetKills (Utilities|Array|Get(acopy) _outactors))
      (:==
        _)
      (:<
        _))
    (Game|OpenLevel(byName) "Level7")
    (Variables|/Game/Blueprints/BP_GameMode.BP_GameMode_C|SetNextLevel (Variables|Default|GetGameMOde) true)))

(fn ConstructionScript)